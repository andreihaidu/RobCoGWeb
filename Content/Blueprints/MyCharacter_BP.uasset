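; Player character Blueprint that handles HUD creation, pausing and pop-up message clearing for a game with hand-based item interaction.
; BeginPlay adds the character HUD to the viewport.
; PauseGame pauses the game, shows the cursor and opens a new main menu widget filled with hard-coded controls help.
; Click and GrabWithTwoHands share one Delay that blanks PopUpMessage after a few seconds; the grab logic itself is not in this graph.
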(event `self.ReceiveBeginPlay`
  (bind _returnvalue (`|CreateWidget` "/Game/Blueprints/MyCharacterHUD_BP.MyCharacterHUD_BP_C"))
  (`UserWidget.AddToViewport` _returnvalue 0))

(event `InputAction|PauseGame`
  (params (Key :type "Key Structure" :default "AnyKey"))
  (:`Pressed`
    (`GameplayStatics.SetGamePaused` true)
    (bind _returnvalue (`|CreateWidget` "/Game/Blueprints/MainMenu_BP.MainMenu_BP_C"))
    (`UserWidget.AddToViewport` _returnvalue 0)
    (set `PlayerController.bShowMouseCursor` true (`GameplayStatics.GetPlayerController` 0))
    (`MultiLineEditableText.SetText` (`/Game/Blueprints/MainMenu_BP.DisplayText` _returnvalue) "*WASD – Character Movement Keys  \n*Click –  Item interraction (pickup or open/close action) \n*Right Click – Pickup stacks \n*TAB – Switch selected hand \n*Arrow Keys – Position adjustment for items held in hand \n*R – Rotation mode and toggle through the axis \n*Mouse Wheel – Rotates the object \n*P – Pause")))

(event `InputAction|Click` :overrideparent false
  (params (Key :type "Key Structure" :default "AnyKey"))
  (:`Pressed`
    (`KismetSystemLibrary.Delay` 4.0 :!label _label)
    (set `self.PopUpMessage` "")))

(event `InputAction|GrabWithTwoHands` :overrideparent false
  (params (Key :type "Key Structure" :default "AnyKey"))
  (:`Pressed`
    (goto _label)))

(fn `UserConstructionScript`)